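; SAMPLE_BAND01_BP is a quest objective actor that the player completes by interacting while inside its trigger box.
; Box overlaps track player presence, and Tick polls the character's Interaction flag.
; On interaction, it finds active quests whose ActorReference is this actor and calls QuestComplete on the player.
; It then notifies AI_king3 actors with a matching quest name through EventQuestComplete and destroys itself upon a match.
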(event OnComponentBeginOverlap(Box)
  (params (OverlappedComponent :type Primitive%20Component%20Object%20Reference) (OtherActor :type Actor%20Object%20Reference) (OtherComp :type Primitive%20Component%20Object%20Reference) (OtherBodyIndex :type Integer) (bFromSweep :type Boolean) (SweepResult :type Hit%20Result%20Structure%20%28by%20ref%29))
  (if (== (Variables|Default|GetCharacter) OtherActor)
    (Variables|Default|SetIsPlayerOnIt true)))

(event OnComponentEndOverlap(Box)
  (params (OverlappedComponent :type Primitive%20Component%20Object%20Reference) (OtherActor :type Actor%20Object%20Reference) (OtherComp :type Primitive%20Component%20Object%20Reference) (OtherBodyIndex :type Integer))
  (if (== (Variables|Default|GetCharacter) OtherActor)
    (Variables|Default|SetIsPlayerOnIt false)))

(event EventBeginPlay
  (bind _asthird_person_character (Utilities|Casting|CastToThirdPersonCharacter (Game|GetPlayerCharacter 0)))
  (Variables|Default|SetCharacter _asthird_person_character))

(event EventTick
  (params (DeltaSeconds :type Float%20%28single-precision%29))
  (if (and (Variables|Default|GetIsPlayerOnIt) (Variables|/Game/ThirdPersonBP/Blueprints/ThirdPersonCharacter.ThirdPersonCharacter_C|GetInteraction (Variables|Default|GetCharacter)))
    (bind _asthird_person_character (Utilities|Casting|CastToThirdPersonCharacter (Game|GetPlayerCharacter 0)))
    (for _array_element (Variables|/Game/ThirdPersonBP/Blueprints/ThirdPersonCharacter.ThirdPersonCharacter_C|GetActiveQuests _asthird_person_character)
      (if (== self (.actorreference (Variables|/Game/BP_Quest.BP_Quest_C|GetQuestInfo _array_element)))
        (Default|QuestComplete _asthird_person_character _array_element)
        (Utilities|FlowControl|Sequence
          (:then_1
            (bind _outactors (Actor|GetAllActorsOfClass "/Game/NPC_peasant_character/NPC-Pack/fbx/unral_better_export/AI_king3.AI_king3_C"))
            (for _array_element_2 _outactors
              (if (Utilities|Enum|Equal(Enum) (.questname (Variables|/Game/BP_Quest.BP_Quest_C|GetQuestInfo _array_element)) (.questname (Variables|/Game/NPC_peasant_character/NPC-Pack/fbx/unral_better_export/AI_king3.AI_king3_C|GetQuestRef _array_element_2)))
                (Default|EventQuestComplete _array_element_2)
                (Actor|DestroyActor)))))))))

(fn ConstructionScript)
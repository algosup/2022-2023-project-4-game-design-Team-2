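; Collectable pickup actor that the third-person character collects by pressing E while inside its collision.
; Overlap enables the actor's input and shows a command prompt widget, gated by a DoOnce that resets when the character leaves.
; Pressing E briefly flashes the prompt as pressed, decrements CollectablesLeft on ThirdPersonGameMode, shows a collectable widget, removes the prompt and destroys the actor.
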(event OnComponentBeginOverlap(collision)
  (params (OverlappedComponent :type Primitive%20Component%20Object%20Reference) (OtherActor :type Actor%20Object%20Reference) (OtherComp :type Primitive%20Component%20Object%20Reference) (OtherBodyIndex :type Integer) (bFromSweep :type Boolean) (SweepResult :type Hit%20Result%20Structure%20%28by%20ref%29))
  (Utilities|FlowControl|DoOnce false
    (:Completed
      (Utilities|Casting|CastToThirdPersonCharacter OtherActor)
      (Input|EnableInput (Game|GetPlayerController 0))
      (bind _returnvalue (UserInterface|CreateWidget "/Game/Object/CommandPromptItem.CommandPromptItem_C"))
      (UserInterface|Viewport|AddtoViewport _returnvalue 0))))

(event OnComponentEndOverlap(collision)
  (params (OverlappedComponent :type Primitive%20Component%20Object%20Reference) (OtherActor :type Actor%20Object%20Reference) (OtherComp :type Primitive%20Component%20Object%20Reference) (OtherBodyIndex :type Integer))
  (bind _returnvalue (Game|GetPlayerController 0))
  (Utilities|Casting|CastToThirdPersonCharacter OtherActor)
  (Input|DisableInput _returnvalue)
  (Widget|RemovefromParent (stale OnComponentBeginOverlap(collision) _returnvalue))
  (Utilities|FlowControl|DoOnce false) ; enters at Reset
)

(event Input|KeyboardEvents|E
  (params (Key :type Key%20Structure :default "None"))
  (:Pressed
    (Variables|/Game/Object/CommandPromptItem.CommandPromptItem_C|SetIsPressed (stale OnComponentBeginOverlap(collision) _returnvalue) true)
    (Utilities|FlowControl|Delay 0.2)
    (Variables|/Game/Object/CommandPromptItem.CommandPromptItem_C|SetIsPressed (stale OnComponentBeginOverlap(collision) _returnvalue) false)
    (bind _asthird_person_game_mode (Utilities|Casting|CastToThirdPersonGameMode (Game|GetGameMode)))
    (bind _result (Math|Integer|DecrementInt (Variables|/Game/ThirdPersonBP/Blueprints/ThirdPersonGameMode.ThirdPersonGameMode_C|GetCollectables%20left _asthird_person_game_mode))
      (:%20%20
        (Variables|/Game/ThirdPersonBP/Blueprints/ThirdPersonGameMode.ThirdPersonGameMode_C|SetCollectables%20left _asthird_person_game_mode _result)
        (bind _returnvalue (UserInterface|CreateWidget "/Game/Object/CollectableWidget.CollectableWidget_C"))
        (UserInterface|Viewport|AddtoViewport _returnvalue 0)
        (Widget|RemovefromParent (stale OnComponentBeginOverlap(collision) _returnvalue))
        (Actor|DestroyActor)))))

(fn ConstructionScript)
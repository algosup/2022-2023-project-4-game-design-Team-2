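; Location trigger actor that completes "reach this place" quests when the ThirdPersonCharacter overlaps its Box.
; On overlap it scans the character's ActiveQuests for entries whose ActorReference is this actor and calls QuestComplete on each match.
; It then searches all actors of five separate AI_king classes in duplicated loops, firing EventQuestComplete on those whose QuestRef shares the completed quest's name.
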(event OnComponentBeginOverlap(Box)
  (params (OverlappedComponent :type Primitive%20Component%20Object%20Reference) (OtherActor :type Actor%20Object%20Reference) (OtherComp :type Primitive%20Component%20Object%20Reference) (OtherBodyIndex :type Integer) (bFromSweep :type Boolean) (SweepResult :type Hit%20Result%20Structure%20%28by%20ref%29))
  (bind _asthird_person_character (Utilities|Casting|CastToThirdPersonCharacter OtherActor))
  (for _array_element (Variables|/Game/ThirdPersonBP/Blueprints/ThirdPersonCharacter.ThirdPersonCharacter_C|GetActiveQuests _asthird_person_character)
    (if (== self (.actorreference (Variables|/Game/BP_Quest.BP_Quest_C|GetQuestInfo _array_element)))
      (Default|QuestComplete _asthird_person_character _array_element)
      (Utilities|FlowControl|Sequence
        (:then_0
          (bind _outactors (Actor|GetAllActorsOfClass "/Game/NPC_peasant_character/NPC-Pack/fbx/unral_better_export/AI_king.AI_king_C"))
          (for _array_element_2 _outactors
            (if (Utilities|Enum|Equal(Enum) (.questname (Variables|/Game/BP_Quest.BP_Quest_C|GetQuestInfo _array_element)) (.questname (Variables|/Game/NPC_peasant_character/NPC-Pack/fbx/unral_better_export/AI_king.AI_king_C|GetQuestRef _array_element_2)))
              (Default|EventQuestComplete _array_element_2))))
        (:then_1
          (bind _outactors_2 (Actor|GetAllActorsOfClass "/Game/NPC_peasant_character/NPC-Pack/fbx/unral_better_export/AI_king2.AI_king2_C"))
          (for _array_element_3 _outactors_2
            (if (Utilities|Enum|Equal(Enum) (.questname (Variables|/Game/BP_Quest.BP_Quest_C|GetQuestInfo _array_element)) (.questname (Variables|/Game/NPC_peasant_character/NPC-Pack/fbx/unral_better_export/AI_king2.AI_king2_C|GetQuestRef _array_element_3)))
              (Default|EventQuestComplete _array_element_3))))
        (:then_2
          (bind _outactors_3 (Actor|GetAllActorsOfClass "/Game/NPC_peasant_character/NPC-Pack/fbx/unral_better_export/AI_king3.AI_king3_C"))
          (for _array_element_4 _outactors_3
            (if (Utilities|Enum|Equal(Enum) (.questname (Variables|/Game/BP_Quest.BP_Quest_C|GetQuestInfo _array_element)) (.questname (Variables|/Game/NPC_peasant_character/NPC-Pack/fbx/unral_better_export/AI_king3.AI_king3_C|GetQuestRef _array_element_4)))
              (Default|EventQuestComplete _array_element_4))))
        (:then_3
          (bind _outactors_4 (Actor|GetAllActorsOfClass "/Game/NPC_peasant_character/NPC-Pack/fbx/unral_better_export/AI_king4.AI_king4_C"))
          (for _array_element_5 _outactors_4
            (if (Utilities|Enum|Equal(Enum) (.questname (Variables|/Game/BP_Quest.BP_Quest_C|GetQuestInfo _array_element)) (.questname (Variables|/Game/NPC_peasant_character/NPC-Pack/fbx/unral_better_export/AI_king4.AI_king4_C|GetQuestRef _array_element_5)))
              (Default|EventQuestComplete _array_element_5))))
        (:then_4
          (bind _outactors_5 (Actor|GetAllActorsOfClass "/Game/NPC_peasant_character/NPC-Pack/fbx/unral_better_export/AI_king5.AI_king5_C"))
          (for _array_element_6 _outactors_5
            (if (Utilities|Enum|Equal(Enum) (.questname (Variables|/Game/BP_Quest.BP_Quest_C|GetQuestInfo _array_element)) (.questname (Variables|/Game/NPC_peasant_character/NPC-Pack/fbx/unral_better_export/AI_king5.AI_king5_C|GetQuestRef _array_element_6)))
              (Default|EventQuestComplete _array_element_6))))))))

(fn ConstructionScript)
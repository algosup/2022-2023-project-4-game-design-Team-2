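; Owl NPC Blueprint that plays ambient idle animations in a random, repeating cycle.
; One second after BeginPlay, it randomly picks between a look-around and a wing-scratch idle, both using crow animation assets.
; Each idle loops on the mesh through PlayAnimation for a random few seconds, then triggers the next random pick.
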(event Custom|DecideNextAction
  ;[1 1 1] random choice
  (switch int (Math|Random|RandomIntegerinRange 0 1)
    (:0
      (CallFunction|Idle1))
    (:1
      (CallFunction|Idle2))))

(event Custom|Idle_1
  ;[1 1 1] Idle
  (Components|Animation|PlayAnimation (Variables|Character|GetMesh) "/Game/NPC_animals/animal_asset/fbx/Animations/owl/ANIM_Crow_IdleLookAround.ANIM_Crow_IdleLookAround" true)
  (Utilities|FlowControl|Delay (Math|Random|RandomFloatinRange 2.0 5.0))
  (CallFunction|DecideNextAction))

(event Custom|Idle_2
  ;[1 1 1] Idle
  (Components|Animation|PlayAnimation (Variables|Character|GetMesh) "/Game/NPC_animals/animal_asset/fbx/Animations/owl/ANIM_Crow_IdleScratchWing.ANIM_Crow_IdleScratchWing" true)
  (Utilities|FlowControl|Delay (Math|Random|RandomFloatinRange 2.0 5.0))
  (CallFunction|DecideNextAction))

(event EventBeginPlay
  (Utilities|FlowControl|Delay 1.0)
  (CallFunction|DecideNextAction))

(fn ConstructionScript)
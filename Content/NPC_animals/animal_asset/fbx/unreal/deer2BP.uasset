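; Deer NPC character Blueprint that wanders on its own with simple ambient behavior, built from events without a Behavior Tree.
; After a short delay at BeginPlay, it randomly picks Idle or Walk, and each loops back to that choice after a random wait.
; Walk sets movement speed and uses AIMoveTo toward a random reachable navmesh point, playing looping mesh animations directly and pausing on success or failure.
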(event Custom|DecideNextAction
  ;[1 1 1] random choice
  (switch int (Math|Random|RandomIntegerinRange 0 1)
    (:0
      (CallFunction|Idle))
    (:1
      (CallFunction|Walk))))

(event Custom|Idle
  ;[1 1 1] Idle
  (Components|Animation|PlayAnimation (Variables|Character|GetMesh) 0 true)
  (Utilities|FlowControl|Delay (Math|Random|RandomFloatinRange 2.0 5.0))
  (CallFunction|DecideNextAction))

(event Custom|Walk
  (bind _self self)
  ;[1 1 1] Walk
  (Variables|/Script/Engine.CharacterMovementComponent|SetMaxWalkSpeed (Variables|Character|GetCharacterMovement) 2e+02)
  (Components|Animation|PlayAnimation (Variables|Character|GetMesh) 0 true)
  (AI|AIMoveTo _self (.RandomLocation (AI|Navigation|GetRandomReachablePointinRadius (Transformation|GetActorLocation _self) 3e+03 0 0)) 0 5.0 false
    (:OnSuccess
      (Components|Animation|PlayAnimation (Variables|Character|GetMesh) 0 true)
      (Utilities|FlowControl|Delay (Math|Random|RandomFloatinRange 4.0 9.0))
      (CallFunction|DecideNextAction))
    (:OnFail
      (Components|Animation|PlayAnimation (Variables|Character|GetMesh) 0 true)
      (Utilities|FlowControl|Delay (Math|Random|RandomFloatinRange 4.0 9.0))
      (CallFunction|DecideNextAction))))

(event EventBeginPlay
  (Utilities|FlowControl|Delay 1.0)
  (CallFunction|DecideNextAction))

(fn ConstructionScript)
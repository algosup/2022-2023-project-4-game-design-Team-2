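; Wolf NPC character Blueprint that runs a simple random wander behavior, starting one second after BeginPlay.
; DecideNextAction picks Idle or Walk at random; Idle loops an animation for a random few seconds, then decides again.
; Walk sets walk speed and loops an animation, but its random-point AIMoveTo chain is disconnected, so the wolf never moves and the cycle stops there.
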(event Custom|DecideNextAction
  ;[1 1 1] random choice
  (switch int (Math|Random|RandomIntegerinRange 0 1)
    (:0
      (CallFunction|Idle))
    (:1
      (CallFunction|Walk))))

(event Custom|Idle
  ;[1 1 1] Idle
  (Components|Animation|PlayAnimation (Variables|Character|GetMesh) 0 true)
  (Utilities|FlowControl|Delay (Math|Random|RandomFloatinRange 2.0 5.0))
  (CallFunction|DecideNextAction))

(event Custom|Walk
  ;[1 1 1] Walk
  (Variables|/Script/Engine.CharacterMovementComponent|SetMaxWalkSpeed (Variables|Character|GetCharacterMovement) 2e+02)
  (Components|Animation|PlayAnimation (Variables|Character|GetMesh) 0 true))

(event EventBeginPlay
  (Utilities|FlowControl|Delay 1.0)
  (CallFunction|DecideNextAction))

(fn ConstructionScript)